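; An exercise actor that loses health over time until it dies.
; On BeginPlay it starts a looping timer at the Tiempo interval that fires QuitarVida.
; Each tick of the timer subtracts Daño from VidaActual through DisminuirVida and prints the remaining health on screen.
; When health reaches zero or below, it prints a death message and destroys itself.
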(event `self.ReceiveBeginPlay`
  (`KismetSystemLibrary.K2_SetTimerDelegate` (delegate `QuitarVida`) (`self.Tiempo`) true))

(event `QuitarVida`
  (`self.Disminuir Vida` (`self.Daño`))
  (`KismetSystemLibrary.PrintString` (`KismetStringLibrary.Conv_DoubleToString` (`self.VidaActual`)) true true (struct :`R` 0.030457 :`G` 1.0 :`A` 1.0) 2.0 "1")
  (if (<= (`self.VidaActual`) 0.0)
    (`KismetSystemLibrary.PrintString` "YOU DIED" true true (struct :`R` 0.782986 :`B` 0.037803 :`A` 1.0))
    (`self.K2_DestroyActor`)))

(fn `Disminuir Vida`
  (params (`Daño` :type "Float (double-precision)"))
  (set `self.VidaActual` (- (`self.VidaActual`) `Daño`)))

(fn `UserConstructionScript`)