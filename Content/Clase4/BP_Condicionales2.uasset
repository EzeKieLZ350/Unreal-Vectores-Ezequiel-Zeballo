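; BP_Condicionales2 is a small Blueprint exercise that demonstrates a conditional on the result of a sum.
; Shortly after BeginPlay, it passes its Num1 and Num2 variables to the Sumar function, which returns their total.
; A branch checks whether the total is positive, then prints it on screen with a "Resultado:" label, switching the text to red for zero or negative results.
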(event `self.ReceiveBeginPlay`
  (`KismetSystemLibrary.Delay` 0.2)
  (bind _resultado (`self.Sumar` (`self.Num 1`) (`self.Num 2`)))
  (if (> _resultado 0)
    (bind _returnvalue (`KismetStringLibrary.Concat_StrStr` "Resultado: \n" (`KismetStringLibrary.Conv_IntToString` _resultado)))
    (`KismetSystemLibrary.PrintString` _returnvalue true true (struct :`G` 0.66 :`B` 1.0 :`A` 1.0) 20.0)
    (else
      (`KismetSystemLibrary.PrintString` _returnvalue true true (struct :`R` 0.887153 :`B` 0.042887 :`A` 1.0) 20.0))))

(fn `Sumar`
  (params (Num1 :type Integer) (Num2 :type Integer))
  (returns (Resultado :type Integer))
  (return (+ Num1 Num2)))

(fn `UserConstructionScript`)