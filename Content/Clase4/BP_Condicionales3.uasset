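; BP_Condicionales3 is a Blueprint exercise in conditionals that simulates an actor losing health over time.
; From BeginPlay, a one-second Delay loop subtracts Daño from Vida, printing the remaining value each pass.
; When Vida reaches zero or below, the actor destroys itself.
; A Sumar function adds two numbers but is not called by the event graph.
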(event `self.ReceiveBeginPlay`
  (bind _vida (`self.Vida`))
  (`KismetSystemLibrary.Delay` 1.0 :!label _label)
  (set `self.Vida` (- (`self.Vida`) (`self.Daño`)))
  (if (<= _vida 0.0)
    (`self.K2_DestroyActor`)
    (else
      (`KismetSystemLibrary.PrintString` (`KismetStringLibrary.Conv_DoubleToString` _vida))
      (goto _label))))

(fn `Sumar`
  (params (Num1 :type Integer) (Num2 :type Integer))
  (returns (Resultado :type Integer))
  (return (+ Num1 Num2)))

(fn `UserConstructionScript`)