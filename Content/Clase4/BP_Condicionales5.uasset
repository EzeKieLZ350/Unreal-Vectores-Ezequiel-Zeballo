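; BP_Condicionales5 is a small Blueprint exercise in conditionals that simulates health draining over time.
; BeginPlay starts a looping half-second timer and stores its handle; each tick fires RestarVida, which subtracts Daño from Vida.
; While Vida stays above zero it prints the value; otherwise it prints a fixed message without the value and clears the timer.
; A Sumar function returns the sum of two inputs but is not called here.
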(event `self.ReceiveBeginPlay`
  (bind _returnvalue (`KismetSystemLibrary.K2_SetTimerDelegate` (delegate `Restar Vida`) 0.5 true))
  (set `self.Handle` _returnvalue))

(event `Restar Vida`
  (bind _vida (`self.Vida`))
  (set `self.Vida` (- (`self.Vida`) (`self.Daño`)))
  (if (<= _vida 0.0)
    (`KismetSystemLibrary.PrintString` "Tu vida es igual a =" true true (struct :`G` 0.66 :`B` 1.0 :`A` 1.0) 5.0)
    (`KismetSystemLibrary.K2_ClearAndInvalidateTimerHandle` (`self.Handle`))
    (else
      (`KismetSystemLibrary.PrintString` (`KismetStringLibrary.Conv_DoubleToString` _vida)))))

(fn `Sumar`
  (params (Num1 :type Integer) (Num2 :type Integer))
  (returns (Resultado :type Integer))
  (return (+ Num1 Num2)))

(fn `UserConstructionScript`)