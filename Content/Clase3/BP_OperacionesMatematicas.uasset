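; BP_OperacionesMatematicas is a Blueprint that demonstrates basic math on a health variable (Vida), using damage (Daño) and a health potion value (PocionDeVida).
; On BeginPlay it subtracts Daño from Vida through the RestarDosNumeros function, stores the result and prints it on screen.
; The addition function SumarDosNumeros and the inline add and subtract variants sit in disconnected nodes that never run.
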(event `self.ReceiveBeginPlay`
  (bind _resta (`self.Restar dos numeros` (`self.Vida`) (`self.Daño`)))
  (bind _output_get (set `self.Vida` _resta))
  (`KismetSystemLibrary.PrintString` (`KismetStringLibrary.Conv_DoubleToString` _output_get) true true (struct :`G` 0.66 :`B` 1.0 :`A` 1.0) 10.0))

(fn `Restar dos numeros`
  (params (`Num 1` :type "Float (double-precision)") (`Num 2` :type "Float (double-precision)"))
  (returns (Resta :type "Float (double-precision)"))
  (return (- `Num 1` `Num 2`)))

(fn `Sumar Dos Numeros`
  (params (`Num 1` :type "Float (double-precision)") (`Num 2` :type "Float (double-precision)"))
  (returns (Sumatoria :type "Float (double-precision)"))
  (return (+ `Num 1` `Num 2`)))

(fn `UserConstructionScript`)